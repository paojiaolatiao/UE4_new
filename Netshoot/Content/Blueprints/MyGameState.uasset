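; Game state that runs a match countdown once exactly two players are in the PlayerArray.
; Tick subtracts delta seconds from Time and separately decrements the 计时 counter by one per frame until it reaches zero.
; When Time drops below zero it sets End and casts the first player controller to MyPlayerController, with nothing wired afterward.
; Both RepNotify handlers and the construction script are empty.
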(event EventTick
  (params (DeltaSeconds :type Float%20%28single-precision%29))
  (Variables|Default|Setstart (== (Utilities|Array|Length (Variables|Default|GetPlayerArray)) 2))
  (if (Variables|Default|Getstart)
    (if (not (Variables|Default|Getend))
      (bind _output_get (Variables|Default|Settime (- (Variables|Default|Gettime) DeltaSeconds)))
      (if (<= (Variables|Default|Get计时) 0)
        _
        (else
          (Variables|Default|Set计时 (- (Variables|Default|Get计时) 1))))
      (if (< _output_get 0.0)
        (Variables|Default|Setend true)
        (Utilities|Casting|CastToMyPlayerController (Game|GetPlayerController 0))))))

(fn ConstructionScript)

(fn OnRepGameStartTimer)

(fn OnRepRandomTimerValue1)