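; BP_Projectile is a projectile actor whose Hit event resolves impacts on characters, their hats and UFOs, then destroys itself.
; Hat-tagged components get knocked off with physics, reduced projectile velocity and random spin.
; Character body hits call ApplyDamage without a wired target; "ufo"-tagged components damage their actor, both spawning hit particles.
; Other impacts print a miss, and the flying-object function 击中飞行物 is not called here.
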(event Collision|EventHit
  (params (MyComp :type Primitive%20Component%20Object%20Reference) (Other :type Actor%20Object%20Reference) (OtherComp :type Primitive%20Component%20Object%20Reference) (bSelfMoved :type Boolean) (HitLocation :type Vector :default "0, 0, 0") (HitNormal :type Vector :default "0, 0, 0") (NormalImpulse :type Vector :default "0, 0, 0") (Hit :type Hit%20Result%20Structure%20%28by%20ref%29))
  (Variables|Default|SetHit%20Location HitLocation)
  (Variables|Default|SetOther Other)
  (Variables|Default|SetOther%20Comp OtherComp)
  ;[0 1 0] Sound
  (Audio|PlaySoundatLocation "/Game/Sounds/SoundCue_Attentuated.SoundCue_Attentuated" (Variables|Default|GetHit%20Location) "0, 0, 0" (Variables|Default|GetVolumeMultiplier) (Math|Random|RandomFloatinRange 0.8 1.2) 0.0 0 0 0)
  (Utilities|Casting|CastToCharacter (Variables|Default|GetOther)
    (:then
      (if (Components|ComponentHasTag (Variables|Default|GetOther%20Comp) "Hat")
        ;[1 1 1] Hit Hat
        (Actor|DestroyActor)
        (Physics|SetSimulatePhysics (Variables|Default|GetOther%20Comp) true)
        (Physics|SetPhysicsLinearVelocity (Variables|Default|GetOther%20Comp) (/ (Variables|/Script/Engine.MovementComponent|GetVelocity (Variables|Default|GetProjectileMovement)) 3.0) false "None")
        (Class|PrimitiveComponent|SetPhysicsAngularVelocityinDegrees (Variables|Default|GetOther%20Comp) (Math|Vector|MakeVector (Math|Random|RandomFloatinRange -7.2e+02 7.2e+02) (Math|Random|RandomFloatinRange -7.2e+02 7.2e+02) (Math|Random|RandomFloatinRange -7.2e+02 7.2e+02)) false "None")
        ;[0 1 0] Sound
        (Audio|PlaySoundatLocation "/Game/Sounds/Randomize_01.Randomize_01" (Variables|Default|GetHit%20Location) "0, 0, 0" (* (Variables|Default|GetVolumeMultiplier) 0.25) 1.0 0.0 0 0 0)
        (else
          ;[1 1 1] Hit Character
          (Game|Damage|ApplyDamage 0 (Math|Random|RandomFloatinRange 1.1e+02 1.1e+02) (Game|GetInstigatorController) 0)
          (Actor|DestroyActor)
          (Effects|SpawnEmitteratLocation "/Game/Effects/P_Hit.P_Hit" (Variables|Default|GetHit%20Location)))))
    (:CastFailed
      (if (Components|ComponentHasTag (Variables|Default|GetOther%20Comp) "ufo")
        (Development|PrintString "命中")
        (Game|Damage|ApplyDamage (Variables|Default|GetOther) (Math|Random|RandomFloatinRange 1e+01 1e+01) (Game|GetInstigatorController) self)
        (Effects|SpawnEmitteratLocation "/Game/Effects/P_Hit.P_Hit" (Variables|Default|GetHit%20Location))
        (Actor|DestroyActor)
        (else
          (Development|PrintText "miss")
          (Actor|DestroyActor))))))

(fn ConstructionScript)

(fn 击中飞行物
  ;[1 1 1] Hit 飞行物体
  (Physics|SetSimulatePhysics (Variables|Default|GetOther%20Comp) true)
  (Development|PrintString "伤害")
  (Game|Damage|ApplyDamage (Variables|Default|GetOther) (Math|Random|RandomFloatinRange 1e+01 1e+01) (Game|GetInstigatorController) self)
  (Effects|SpawnEmitteratLocation "/Game/Effects/P_Hit.P_Hit" (Variables|Default|GetHit%20Location)))